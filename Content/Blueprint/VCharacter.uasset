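; Player character Blueprint with look and movement controls plus a car-entry sequence.
; Pressing EnterCar while CanEnterCar is set loops over all VCar actors, issues SimpleMoveToLocation to each one's door point and sets PlayEnterCarAnim, which blocks movement input.
; A separate StartEntering event, not called within this graph, plays the Adam_AM montage's EnterCar section and disables actor collision.
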(event `InputAxis|LookUp`
  (params (AxisValue :type "Float (single-precision)"))
  ;[1 1 1] Turn
  (`self.AddControllerPitchInput` AxisValue))

(event `InputAxis|Turn`
  (params (AxisValue :type "Float (single-precision)"))
  ;[1 1 1] Turn
  (`self.AddControllerYawInput` AxisValue))

(event `InputAxis|MoveForward`
  (params (AxisValue :type "Float (single-precision)"))
  ;[1 1 1] Movement
  (if (not (`self.bPlayEnterCarAnim`))
    (`self.AddMovementInput` (`KismetMathLibrary.GetForwardVector` (`KismetMathLibrary.MakeRotator` 0.0 0.0 (.yaw (`self.GetControlRotation`)))) AxisValue)))

(event `InputAxis|MoveRight`
  (params (AxisValue :type "Float (single-precision)"))
  ;[1 1 1] Movement
  (if (not (`self.bPlayEnterCarAnim`))
    (`self.AddMovementInput` (`KismetMathLibrary.GetRightVector` (`KismetMathLibrary.MakeRotator` 0.0 0.0 (.yaw (`self.GetControlRotation`)))) AxisValue)))

(event `InputAction|EnterCar`
  (params (Key :type "Key Structure"))
  ;[1 1 1] Enter Car
  (:`Pressed`
    (if (`self.bCanEnterCar`)
      (bind _outactors (`GameplayStatics.GetAllActorsOfClass` "/Game/Blueprint/VCar.VCar_C"))
      (for _array_element _outactors
        (bind _asvcar (cast `/Game/Blueprint/VCar` _array_element))
        (`AIBlueprintHelperLibrary.SimpleMoveToLocation` (`self.GetController`) (`SceneComponent.K2_GetComponentLocation` (`/Game/Blueprint/VCar.DoorLocatEnter` _asvcar)))
        (set `self.bPlayEnterCarAnim` true)))))

(event `StartEntering`
  ;[1 1 1] Start Entering Car
  (`|PlayMontage` (`self.Mesh`) "/Game/Meshes/Character/Anim/Adam_AM.Adam_AM" 1.0 0.0 "EnterCar"
    (:`then`
      (`self.SetActorEnableCollision` false))))

(fn `UserConstructionScript`)