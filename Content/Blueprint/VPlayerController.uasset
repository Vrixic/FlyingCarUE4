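; Player controller that switches possession between the VCharacter and a VCar, and owns the controls menu widget.
; BeginPlay finds both actors, binds the enter and exit car events, and shows the menu, whose animation replays on the Menu input.
; Entering possesses the car; exiting possesses the character, then destroys and respawns it at the car's exit location, at zero height with yaw relative to the vehicle.
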(event `self.ReceiveBeginPlay`
  (bind _outactors (`GameplayStatics.GetAllActorsOfClass` "/Game/Blueprint/VCharacter.VCharacter_C"))
  (for _array_element _outactors
    (`/Engine/EditorBlueprintResources/StandardMacros.IsValid` _array_element
      (:`Is Valid`
        (set `self.PlayerCharacter` _array_element)
        (bind _outactors_2 (`GameplayStatics.GetAllActorsOfClass` "/Game/Blueprint/VCar.VCar_C"))
        (for _array_element_2 _outactors_2
          (`/Engine/EditorBlueprintResources/StandardMacros.IsValid` _array_element_2
            (:`Is Valid`
              (set `self.Vehicle` _array_element_2)
              (add `self.EnterCar` (delegate `EnterCar_Event`))
              (add `self.ExitCar` (delegate `ExitCar_Event`))
              (bind _returnvalue (`|CreateWidget` "/Game/Blueprint/HUDS/Controls_WBP.Controls_WBP_C"))
              (bind _output_get (set `self.Menu_WBP` _returnvalue))
              (`UserWidget.AddToViewport` _output_get 0)
              (`Widget.SetVisibility` _output_get "Visible")
              (`/Game/Blueprint/HUDS/Controls_WBP.PlayMovingAnimation` _output_get))))))))

(event `ExitCar_Event`
  (bind _vehicle (`self.Vehicle`))
  (bind _playercharacter (`self.PlayerCharacter`))
  (bind (_returnvalue_x _returnvalue_y) (`KismetMathLibrary.BreakVector` (`SceneComponent.K2_GetComponentLocation` (`/Game/Blueprint/VCar.ExitLocation` _vehicle))))
  (bind (_returnvalue_roll _returnvalue_pitch _returnvalue_yaw) (`KismetMathLibrary.BreakRotator` (`SceneComponent.K2_GetComponentRotation` (`VehicleSystemBase.VehicleMesh` _vehicle))))
  (`self.Possess` _playercharacter)
  (`self.K2_DestroyActor` _playercharacter)
  (bind _returnvalue (`|SpawnActorFromClass` (`GameplayStatics.GetObjectClass` _playercharacter) (`KismetMathLibrary.MakeTransform` (`KismetMathLibrary.MakeVector` _returnvalue_x _returnvalue_y) (`KismetMathLibrary.MakeRotator` 0.0 0.0 (- _returnvalue_yaw 90.0))) "Undefined" "OverrideRootScale" null null))
  (set `self.PlayerCharacter` _returnvalue))

(event `EnterCar_Event`
  (bind _vehicle (`self.Vehicle`))
  (`self.Possess` _vehicle)
  (`/Game/Blueprint/VCar.PlayerEnteredCar` _vehicle))

(event `InputAction|Menu`
  (params (Key :type "Key Structure"))
  (:`Pressed`
    (`/Game/Blueprint/HUDS/Controls_WBP.PlayMovingAnimation` (`self.Menu_WBP`))))

(fn `CheckPlayerValidity`
  (params (PC :type "/Game/Blueprint/VCharacter Object Reference"))
  (`/Engine/EditorBlueprintResources/StandardMacros.IsValid` PC
    (:`Is Not Valid`
      (bind _outactors (`GameplayStatics.GetAllActorsOfClass` "/Game/Blueprint/VCharacter.VCharacter_C"))
      (for _array_element _outactors
        (`/Engine/EditorBlueprintResources/StandardMacros.IsValid` _array_element
          (:`Is Valid`
            (set `self.PlayerCharacter` _array_element))
          (:`Is Not Valid`
            (`self.CheckPlayerValidity` (`self.PlayerCharacter`))))))))

(fn `UserConstructionScript`)